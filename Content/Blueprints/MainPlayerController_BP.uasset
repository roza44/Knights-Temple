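; Player controller Blueprint that adds animated transitions to the pause menu when it is shown and removed.
; Both events call the parent implementation, then cast the menu widget to PauseMenu and play its PauseMenuAnimation, forward on display and in reverse on removal.
; On removal, a short delay lets the reverse animation play before the widget is set to Hidden.
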(event `self.DisplayPauseMenu`
  (`parent.DisplayPauseMenu`)
  (bind _aspause_menu (cast `/Game/HUD/PauseMenu` (`self.PauseMenu`)))
  (`UserWidget.PlayAnimation` _aspause_menu (`/Game/HUD/PauseMenu.PauseMenuAnimation` _aspause_menu) 0.0 1 "Forward" 1.0 false))

(event `self.RemovePauseMenu`
  (`parent.RemovePauseMenu`)
  (bind _aspause_menu (cast `/Game/HUD/PauseMenu` (`self.PauseMenu`)))
  (`UserWidget.PlayAnimation` _aspause_menu (`/Game/HUD/PauseMenu.PauseMenuAnimation` _aspause_menu) 0.0 1 "Reverse" 1.0 false)
  (`KismetSystemLibrary.Delay` 0.2)
  (`Widget.SetVisibility` (`self.PauseMenu`) "Hidden"))

(fn `UserConstructionScript`)